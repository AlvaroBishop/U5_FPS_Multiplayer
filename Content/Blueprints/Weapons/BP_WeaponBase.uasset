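; Base weapon actor that acts as a physics-simulated pickup in the world and offers itself to players who overlap it.
; When a Player-tagged actor enters its collision sphere, the server fetches the player reference and compares weapon types against that player's inventory.
; It registers as an overlapped weapon only if no type matches, using the player's CanLootWeapon flag, which resets after a blocked attempt.
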(event `self.ReceiveBeginPlay`
  (`PrimitiveComponent.SetSimulatePhysics` (`self.Weapon`) true))

(event `self.SphereCollision.OnComponentBeginOverlap`
  (params (OverlappedComponent :type "PrimitiveComponent Object Reference") (OtherActor :type "Actor Object Reference") (OtherComp :type "PrimitiveComponent Object Reference") (OtherBodyIndex :type Integer) (bFromSweep :type Boolean) (SweepResult :type "HitResult Structure (by ref)"))
  (if (`self.ActorHasTag` OtherActor "Player")
    (`/Engine/EditorBlueprintResources/ActorMacros.Switch Has Authority`
      (:`Authority`
        (bind _player (message `/Game/Blueprints/Interfaces/INT_Player_Base.GetPlayerRef` OtherActor))
        (for _array_element (`/Game/Blueprints/Player/BP_Player_Base.WeaponInventory` _player)
          (if (`|EnumEquality` (`.Type_5_CE83240042E29317C52FB4A224AD56B9` (break `/Game/Blueprints/Structure/ST_WeaponInfo` (`/Game/Blueprints/Libraries/BP_FunctionLibrary.f_GetWeaponInfo` (`/Game/Blueprints/Weapons/BP_WeaponBase.WeaponName` _array_element)))) (`.Type_5_CE83240042E29317C52FB4A224AD56B9` (break `/Game/Blueprints/Structure/ST_WeaponInfo` (`/Game/Blueprints/Libraries/BP_FunctionLibrary.f_GetWeaponInfo` (`self.WeaponName`)))))
            (set `/Game/Blueprints/Player/BP_Player_Base.bCanLootWeapon` false _player)
            (break)))
        (if (`/Game/Blueprints/Player/BP_Player_Base.bCanLootWeapon` _player)
          (`/Game/Blueprints/Player/BP_Player_Base.AddOverlappedWeapon` _player self)
          (else
            (set `/Game/Blueprints/Player/BP_Player_Base.bCanLootWeapon` true _player)))))))

(fn `UserConstructionScript`)