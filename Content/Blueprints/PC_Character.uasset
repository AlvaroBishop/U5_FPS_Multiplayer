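; Player controller that sets up the player's HUD at BeginPlay, showing main and crosshair widgets with game-only input and a hidden cursor.
; SpawnPlayer spawns no pawn; it and ShowHideWidget forward to CL_-prefixed events that perform the UI work.
; An enum-style switch lazily creates, caches and adds each widget to the viewport, or removes it from its parent.
; Team selection widget branches exist but are unreachable.
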(event `self.ReceiveBeginPlay`
  (`self.SpawnPlayer`))

(event `SpawnPlayer`
  (`self.CL_SpawnPlayer`))

(event `CL_SpawnPlayer`
  (`self.ShowHideWidget` true)
  (`self.ShowHideWidget` true "NewEnumerator1")
  (`WidgetBlueprintLibrary.SetInputMode_GameOnly` self)
  (set `self.bShowMouseCursor` false))

(event `ShowHideWidget`
  (params (Show :type Boolean) (Widget :type "/Game/Blueprints/Enums/E_GameWidgets Enum" :default "NewEnumerator0"))
  (`self.CL_ShowHideWidget` Show Widget))

(event `CL_ShowHideWidget`
  (params (Show :type Boolean) (Widget :type "/Game/Blueprints/Enums/E_GameWidgets Enum" :default "NewEnumerator0"))
  (if Show
    (`self.f_ShowWidget` Widget)
    (else
      (`self.f_HideWidget` Widget))))

(fn `f_HideWidget`
  (params (Widgets :type "/Game/Blueprints/Enums/E_GameWidgets Enum" :default "NewEnumerator0"))
  (switch `/Game/Blueprints/Enums/E_GameWidgets` Widgets
    (:`NewEnumerator0`
      (bind _wb_main (`self.WB_Main`)
        (:`then`
          (`Widget.RemoveFromParent` _wb_main))
        (:`else`)))
    (:`NewEnumerator1`
      (bind _wb_crosshair (`self.WB_Crosshair`)
        (:`then`
          (`Widget.RemoveFromParent` _wb_crosshair))
        (:`else`)))))

(fn `f_ShowWidget`
  (params (Widget :type "/Game/Blueprints/Enums/E_GameWidgets Enum" :default "NewEnumerator0"))
  (`KismetSystemLibrary.PrintString` "show widget")
  (switch `/Game/Blueprints/Enums/E_GameWidgets` Widget
    (:`NewEnumerator0`
      (`self.WB_Main`
        (:`then`
          _)
        (:`else`
          (bind _returnvalue (`|CreateWidget` "/Game/UI/WB_Main.WB_Main_C"))
          (bind _output_get (set `self.WB_Main` _returnvalue))))
      (`UserWidget.AddToViewport` _output_get 0))
    (:`NewEnumerator1`
      (`self.WB_Crosshair`
        (:`then`
          _)
        (:`else`
          (bind _returnvalue_2 (`|CreateWidget` "/Game/UI/WB_Crosshair.WB_Crosshair_C"))
          (bind _output_get_2 (set `self.WB_Crosshair` _returnvalue_2))))
      (`UserWidget.AddToViewport` _output_get_2 0))))

(fn `GetPlayerControllerRef`
  (returns (PlayerController :type "/Game/Blueprints/PC_Character Object Reference"))
  (return self))

(fn `UserConstructionScript`)