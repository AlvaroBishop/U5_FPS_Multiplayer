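; Networked AI rifleman that wanders, engages pawns it senses and reports its death for an enemies-left check.
; A two-second loop resumes wandering unless a target was sensed; engagement randomly picks approach or sideways movement while shooting.
; Server-named events drive timer-based, randomly spread line-trace fire with headshot damage and reloads, while multicasts play AK47 data-driven effects and montages.
; Damage depletes health until OnRep death triggers ragdoll and stops firing.
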(event `self.ReceiveBeginPlay`
  ;[0.4453 1 0.2114] BeignPlay
  (set `self.CurrentHealth` (`self.MaxHealth`))
  (`self.Search Around`)
  (`KismetSystemLibrary.Delay` 2.0 :!label _label)
  (`self.Search Around`)
  (set `self.bHasSeenTarget` false)
  (goto _label))

(event `Search Around`
  ;[1 1 1] SearchLoop
  (if (not (`self.bHasSeenTarget`))
    (`self.SRV_ShootWeapon` false)
    (`|AIMoveTo` self (`NavigationSystemV1.K2_GetRandomReachablePointInRadius` (`self.K2_GetActorLocation`) 2000.0 null null) null 300.0)))

(event `SRV_CalculateAimDirection`
  (`self.f_CalculateAimDirection`))

(event `self.ReceiveAnyDamage`
  (params (Damage :type "Float (single-precision)") (DamageType :type "DamageType Object Reference") (InstigatedBy :type "Controller Object Reference") (DamageCauser :type "Actor Object Reference"))
  (bind _currenthealth (`self.CurrentHealth`))
  ;[0 0 0 1 25] Death
  (`KismetSystemLibrary.PrintString` (`KismetStringLibrary.Conv_DoubleToString` _currenthealth) :!enabledstate Disabled)
  (bind _output_get (set `self.CurrentHealth` (`KismetMathLibrary.FClamp` (- _currenthealth Damage) 0.0 (`self.MaxHealth`))))
  (if (== _output_get 0.0)
    (`self.Death` true)))

(event `Death`
  (params (bIsDeath :type Boolean))
  ;[0 0 0 1 25] Death
  (`self.SRV_Death` bIsDeath))

(event `SRV_Death`
  (params (bIsDeath :type Boolean))
  ;[0 0 0 1 25] Death
  (set `self.bIsDeath` bIsDeath))

(event `self.PawnSensing.OnSeePawn`
  (params (Pawn :type "Pawn Object Reference"))
  ;[1 0.2904 0.3303] OnPawnSensing
  (set `self.bHasSeenTarget` true :!label _label_2)
  (bind _player (message `/Game/Blueprints/Interfaces/INT_Player_Base.GetPlayerRef` Pawn))
  (if (not (`/Game/Blueprints/Player/BP_Player_Base.bIsDeath` _player))
    (`self.ChaseTarget` _player)))

(event `self.PawnSensing.OnHearNoise`
  (params (Instigator :type "Pawn Object Reference") (Location :type "Vector Structure (by ref)") (Volume :type "Float (single-precision)"))
  ;[1 0.2904 0.3303] OnPawnSensing
  (goto _label_2))

(event `ChaseTarget`
  (params (TargetActor :type "Actor Object Reference"))
  (bind _returnvalue (+ (`SceneComponent.GetRightVector` (`self.Mesh`)) 500.0))
  ;[1 1 1] ChaseTarget
  (if (not (`self.bIsDead?`))
    (switch `int` (`KismetMathLibrary.RandomIntegerInRange` 0 1)
      (:`0`
        (set `CharacterMovementComponent.bOrientRotationToMovement` true (`self.CharacterMovement`))
        (if (not (`self.bIsReloading`))
          (`self.SRV_ShootWeapon` true)
          (else
            (`self.SRV_ShootWeapon` false)))
        (`|AIMoveTo` self (0.0 0.0 0.0) TargetActor 450.0))
      (:`1`
        (set `CharacterMovementComponent.bOrientRotationToMovement` false (`self.CharacterMovement`))
        (`self.SRV_ShootWeapon` true)
        (`|AIMoveTo` self (`KismetMathLibrary.SelectVector` _returnvalue (* _returnvalue -1.0) (`KismetMathLibrary.RandomBool`)) null 450.0)))))

(event `SRV_ShootWeapon`
  (params (bShootWeapon :type Boolean))
  (bind _shootweaponhandle (`self.ShootWeaponHandle`))
  ;[0 0.341 1] Shoot
  (if bShootWeapon
    (`/Engine/EditorBlueprintResources/StandardMacros.DoOnce` false :!label _label_3
      (:`Completed`
        (`self.InitialWeaponShot`)
        (switch `/Game/Blueprints/Enums/E_WeaponTypes` "NewEnumerator2"
          (:`NewEnumerator2`
            (bind _returnvalue (`KismetSystemLibrary.K2_SetTimerDelegate` (delegate `ShootWeaponLoop`) (`.ShootingSpeed_18_AC1735BA444033FE8295C2813C98B0B7` (break `/Game/Blueprints/Structure/ST_WeaponInfo` (`/Game/Blueprints/Libraries/BP_FunctionLibrary.f_GetWeaponInfo` "AK47"))) true))
            (set `self.ShootWeaponHandle` _returnvalue)))))
    (else
      (if (`KismetSystemLibrary.K2_IsValidTimerHandle` _shootweaponhandle)
        (`KismetSystemLibrary.K2_ClearAndInvalidateTimerHandle` _shootweaponhandle))
      (`self.CanShootAgain`))))

(event `CanShootAgain`
  ;[0 0.341 1] Shoot
  (goto _label_3 :!via `Reset`))

(event `InitialWeaponShot`
  (bind (_startlocation _endlocation) (`self.f_GetBulletLineTraceLocations` 20000.0))
  (bind _returnvalue (`SceneComponent.GetSocketLocation` (`self.Weapon`) "S_Muzzle"))
  (bind _x (.x _endlocation))
  (bind _y (.y _endlocation))
  (bind _z (.z _endlocation))
  ;[0 0.341 1] Shoot
  (`|ExecutionSequence` :!label _label_4
    (:`then_0`
      (if (and (not (`self.bIsReloading`)) (not (`self.f_IsOutOfAmmo`)))
        (`self.MC_ShootWeapon` _returnvalue true)
        (`self.f_SubstractAmmoFromMag` 1)
        (else
          (`self.MC_ShootWeapon` _returnvalue (!= (`self.CurrentExtraAmmo`) 0)))))
    (:`then_1`
      (if (and (not (`self.bIsReloading`)) (not (`self.f_IsOutOfAmmo`)))
        (bind (_outhit _returnvalue_2) (`KismetSystemLibrary.LineTraceSingle` _startlocation (`KismetMathLibrary.MakeVector` (`KismetMathLibrary.RandomFloatInRange` (- _x 500.0) (+ _x 500.0)) (`KismetMathLibrary.RandomFloatInRange` (- _y 500.0) (+ _y 500.0)) (`KismetMathLibrary.RandomFloatInRange` (- _z 2500.0) (+ _z 0.0))) "TraceTypeQuery1" false (`|MakeArray` self :!type "Actor Object Reference") "ForDuration" true (struct :`R` 1.0 :`B` 0.086574 :`A` 1.0)))
        (if _returnvalue_2
          (bind (_bblockinghit _binitialoverlap _time _distance _location _impactpoint _normal _impactnormal _physmat _hitactor _hitcomponent _hitbonename) (`GameplayStatics.BreakHitResult` _outhit))
          (if _bblockinghit
            (`self.MC_BulletImpact` _location _hitactor)
            (if (or (`self.ActorHasTag` _hitactor "Player") (`self.ActorHasTag` _hitactor "AI"))
              (`KismetSystemLibrary.PrintString` "Hit" :!enabledstate Disabled)
              (switch `name` _hitbonename
                (:`Default`
                  (`GameplayStatics.ApplyDamage` _hitactor 10.0))
                (:`head`
                  (`GameplayStatics.ApplyDamage` _hitactor 20.0))))))))
    (:`then_2`
      (if (and (`self.f_IsOutOfAmmo`) (not (`self.bIsReloading`)) (`self.f_HasExtraAmmo`))
        (`self.SetIsReloadingWeapon` true)))))

(event `ShootWeaponLoop`
  ;[0 0.341 1] Shoot
  (goto _label_4))

(event `MC_ShootWeapon`
  (params (Location :type "Vector Structure") (bHasAmmo :type Boolean))
  (bind ((`ShootAnimation_36_192801EC4EE7B8D195FA939E61269D84` _shootanimation) (`ShootingSFX_20_301C12A04C31CC3CAC81F3851B658FBB` _shootingsfx) (`OutOfAmmoSFX_39_E9784ABE4A6AAD136C60DCB5A6E83023` _outofammosfx) (`MuzzleFlash_19_BD63A8F2462A79DE7E1337ACFCCAA5D8` _muzzleflash)) (break `/Game/Blueprints/Structure/ST_WeaponInfo` (`/Game/Blueprints/Libraries/BP_FunctionLibrary.f_GetWeaponInfo` "AK47")))
  ;[0 0 0 1 25] Muzzle Flash
  (if bHasAmmo
    (if (and (not (`self.f_IsOutOfAmmo`)) (not (`self.bIsReloading`)))
      (`|PlayMontage` (`self.Mesh`) _shootanimation
        (:`then`
          (bind _returnvalue (`GameplayStatics.SpawnEmitterAttached` _muzzleflash (`self.Weapon`) "S_Muzzle" (0.0 0.0 0.0) (struct) (0.5 0.5 0.5)))
          (set `self.MuzzleFlashEmitter` _returnvalue)
          (`GameplayStatics.PlaySoundAtLocation` _shootingsfx Location (struct) 1.0 1.0 0.0 null null null null))))
    (else
      (`GameplayStatics.PlaySoundAtLocation` _outofammosfx Location (struct) 1.0 1.0 0.0 null null null null))))

(event `MC_BulletImpact`
  (params (HitLocation :type "Vector Structure") (HitActor :type "Actor Object Reference"))
  (bind ((`BulletImpactSFX_47_DAC3637442641B4EE60C1687D8E9DBC5` _bulletimpactsfx) (`BulletImpactPlayerSFX_50_16481157498D20B1FB61AB8F938172AC` _bulletimpactplayersfx) (`BulletImpactVFX_46_C5B972E14D5A30A28E709580E3B150BE` _bulletimpactvfx) (`BulletImpactPlayerVFX_52_16D2DCD34A0C02811F092686656FB197` _bulletimpactplayervfx)) (break `/Game/Blueprints/Structure/ST_WeaponInfo` (`/Game/Blueprints/Libraries/BP_FunctionLibrary.f_GetWeaponInfo` "AK47")))
  (bind _returnvalue (or (`self.ActorHasTag` HitActor "Player") (`self.ActorHasTag` HitActor "AI")))
  ;[0.4763 1 0.4729] BulletImpact
  (`GameplayStatics.SpawnEmitterAtLocation` (select `bool` _returnvalue :`false` _bulletimpactvfx :`true` _bulletimpactplayervfx) HitLocation)
  (`GameplayStatics.PlaySoundAtLocation` (select `bool` _returnvalue :`false` _bulletimpactsfx :`true` _bulletimpactplayersfx :!type "SoundBase Object Reference") HitLocation (struct) 1.0 1.0 0.0 null null null null)
  (`GameplayStatics.SpawnDecalAtLocation` null (1.0 1.0 1.0)))

(event `SetIsReloadingWeapon`
  (params (bIsReloading :type Boolean))
  ;[0.7318 0 1] Reload
  (`self.SRV_SetIsReloadingWeapon` bIsReloading))

(event `SRV_SetIsReloadingWeapon`
  (params (bIsReloading :type Boolean))
  (bind ((`MaxammoinMag_28_E52FBEE7475CBEB75AE0E29C5AA9FBBA` _maxammoinmag)) (break `/Game/Blueprints/Structure/ST_WeaponInfo` (`/Game/Blueprints/Libraries/BP_FunctionLibrary.f_GetWeaponInfo` "AK47")))
  (bind ((`ReloadAnimation_32_F61EFFEA42D2F77AA4585DA99DF66E60` _reloadanimation) (`MagName_61_BA76BA1A4487237604B7AEA27E0BC752` _magname)) (break `/Game/Blueprints/Structure/ST_WeaponInfo` (`/Game/Blueprints/Libraries/BP_FunctionLibrary.f_GetWeaponInfo` "AK47")))
  ;[0.7318 0 1] Reload
  (bind _output_get (set `self.bIsReloading` bIsReloading))
  (if _output_get
    (`self.MC_SetIsReloadingWeapon` _reloadanimation _magname)
    (elif (>= (+ (`self.CurrentExtraAmmo`) (`self.CurrentAmmoInMag`)) _maxammoinmag)
      (set `self.CurrentExtraAmmo` (`KismetMathLibrary.Clamp` (- (`self.CurrentExtraAmmo`) (- _maxammoinmag (`self.CurrentAmmoInMag`))) 0 (`self.CurrentExtraAmmo`)))
      (set `self.CurrentAmmoInMag` _maxammoinmag)
      (else
        (set `self.CurrentAmmoInMag` (+ (`self.CurrentExtraAmmo`) (`self.CurrentAmmoInMag`)))
        (set `self.CurrentExtraAmmo` 0)))))

(event `MC_SetIsReloadingWeapon`
  (params (AnimMontage :type "AnimMontage Object Reference") (MagName :type Name))
  ;[0.7318 0 1] Reload
  (bind _notifyname (`|PlayMontage` (`self.Mesh`) AnimMontage)
    (:`OnCompleted`
      (`self.SRV_SetIsReloadingWeapon` false))
    (:`OnNotifyBegin`
      (if (== _notifyname "ClipOut")
        (`SkinnedMeshComponent.HideBoneByName` (`self.Weapon`) MagName "PBO_None")
        (else
          (`SkinnedMeshComponent.UnHideBoneByName` (`self.Weapon`) MagName))))))

(fn `f_CalculateAimDirection`
  (`/Engine/EditorBlueprintResources/ActorMacros.Switch Has Authority`
    (:`Authority`
      _)
    (:`Remote`
      (`self.SRV_CalculateAimDirection`)))
  (set `self.AimDirection` (.pitch (`KismetMathLibrary.NormalizedDeltaRotator` (`self.GetControlRotation`) (`self.K2_GetActorRotation`)))))

(fn `f_GetBulletLineTraceLocations`
  (params (DistanceMultiplier :type "Float (single-precision)"))
  (returns (StartLocation :type "Vector Structure") (EndLocation :type "Vector Structure"))
  (bind _weapon (`self.Weapon`))
  (bind _returnvalue (`SceneComponent.K2_GetComponentLocation` _weapon))
  (return _returnvalue (+ _returnvalue (* (`SceneComponent.GetRightVector` _weapon) DistanceMultiplier))))

(fn `f_HasExtraAmmo`
  (returns (ReturnValue :type Boolean))
  (return (!= (`self.CurrentExtraAmmo`) 0)))

(fn `f_IsOutOfAmmo`
  (returns (ReturnValue :type Boolean))
  (return (== (`self.CurrentAmmoInMag`) 0)))

(fn `f_SubstractAmmoFromMag`
  (params (AmmoToSubstract :type Integer))
  (set `self.CurrentAmmoInMag` (`KismetMathLibrary.Clamp` (- (`self.CurrentAmmoInMag`) AmmoToSubstract) 0 (`.MaxammoinMag_28_E52FBEE7475CBEB75AE0E29C5AA9FBBA` (break `/Game/Blueprints/Structure/ST_WeaponInfo` (`/Game/Blueprints/Libraries/BP_FunctionLibrary.f_GetWeaponInfo` "AK47"))))))

(fn `OnRep_bIsDeath`
  (bind _mesh (`self.Mesh`))
  (bind _mesh_2 (`self.Mesh`))
  (if (`self.bIsDeath`)
    (`PrimitiveComponent.SetCollisionEnabled` (`self.CapsuleComponent`) "NoCollision")
    (`PrimitiveComponent.SetCollisionEnabled` _mesh "PhysicsOnly")
    (`PrimitiveComponent.SetSimulatePhysics` _mesh true)
    (`SkeletalMeshComponent.PlayAnimation` _mesh null false)
    (`CharacterMovementComponent.DisableMovement` (`self.CharacterMovement`))
    (set `self.bIsDead?` true)
    (`self.CheckEnemiesLeft`)
    (`self.SRV_ShootWeapon` false)
    (else
      (`PrimitiveComponent.SetSimulatePhysics` _mesh_2 false)
      (`PrimitiveComponent.SetCollisionEnabled` _mesh_2 "QueryOnly")
      (`PrimitiveComponent.SetCollisionEnabled` (`self.CapsuleComponent`) "QueryAndPhysics")
      (`CharacterMovementComponent.SetMovementMode` (`self.CharacterMovement`) "MOVE_None" 0)
      (`SkeletalMeshComponent.SetAnimationMode` _mesh_2 "AnimationBlueprint")
      (`SkeletalMeshComponent.SetAnimInstanceClass` _mesh_2 "/Game/Blueprints/Player/Animations/AnimBP_Player.AnimBP_Player_C")
      (`SceneComponent.K2_AttachToComponent` _mesh_2 (`self.CapsuleComponent`) "None" "SnapToTarget" "SnapToTarget" "SnapToTarget" true))))

(fn `UserConstructionScript`)