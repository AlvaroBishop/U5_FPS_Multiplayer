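; Base game instance, kept with the main menu, that hosts multiplayer servers through Advanced Sessions.
; CreateServer builds a session advertising server name, selected map, language and LAN flag, using the requested slot count.
; On success it opens the level matching SelectedGameMap as a listen server; failure is not handled.
; GetGameInstanceRef simply returns the instance itself.
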(event `CreateServer`
  (params (`Server Name` :type String) (`Amount Of Slots` :type Integer) (bUseLAN :type Boolean) (`Server Language` :type String))
  (`CreateSessionCallbackProxyAdvanced.CreateAdvancedSession` (`|MakeArray` (`AdvancedSessionsLibrary.MakeLiteralSessionPropertyString` "ServerName" `Server Name`) (`AdvancedSessionsLibrary.MakeLiteralSessionPropertyString` "ServerMap" (`|GetEnumeratorNameAsString` (`self.SelectedGameMap`))) (`AdvancedSessionsLibrary.MakeLiteralSessionPropertyString` "ServerLanguage" `Server Language`) (`AdvancedSessionsLibrary.MakeLiteralSessionPropertyBool` "IsUsingLan" bUseLAN)) (`GameplayStatics.GetPlayerController` 0) `Amount Of Slots` 0 bUseLAN
    (:`OnSuccess`
      (`GameplayStatics.OpenLevelBySoftObjectPtr` (select `/Game/Blueprints/Enums/E_GameMaps` (`self.SelectedGameMap`) :`NewEnumerator0` "/Game/Maps/MAP_Main.MAP_Main" :`NewEnumerator1` "/Game/Maps/MAP_Main2.MAP_Main2" :`NewEnumerator2` "/Game/Maps/MAP_Main3.MAP_Main3" :`NewEnumerator3` "/Game/Maps/MAP_Main4.MAP_Main4" :!type "World Soft Object Reference") true "listen"))))

(fn `GetGameInstanceRef`
  (returns (GameInstance :type "/Game/Blueprints/MainMenu/GI_Base Object Reference"))
  (return self))